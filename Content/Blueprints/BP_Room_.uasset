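; BP_Room_ is a room actor with an easy and a hard exit trigger that populate the stretch ahead when the player character overlaps one.
; ExitLight spawns slow-moving BP_First actors; ExitHard spawns more with Move1, plus a BP_Survive.
; Both add an equal number of randomly placed static catches, then destroy both exit triggers so the choice happens once.
; The Stop1 and Stop2 triggers each spawn a BP_Block behind the room's origin.
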(event OnComponentBeginOverlap(ExitHard)
  (params (OverlappedComponent :type Primitive%20Component%20Object%20Reference) (OtherActor :type Actor%20Object%20Reference) (OtherComp :type Primitive%20Component%20Object%20Reference) (OtherBodyIndex :type Integer) (bFromSweep :type Boolean) (SweepResult :type Hit%20Result%20Structure%20%28by%20ref%29))
  (bind _returnvalue (Transformation|GetActorLocation))
  (bind _x (Math|Vector|BreakVector _returnvalue))
  (Utilities|Casting|CastToBP_ThirdPersonCharacter OtherActor)
  (Variables|Default|SetCatchCount 8)
  (for _index (range 0 (- (Variables|Default|GetCatchCount) 1))
    (bind _returnvalue_2 (Game|SpawnActorfromClass "/Game/Blueprints/BP_First.BP_First_C" (Math|Transform|MakeTransform (Math|Vector|MakeVector (Math|Random|RandomFloatinRange (+ _x 1.15e+03) (+ _x 2.65e+03)) -3.2e+02 35.0) "0, 0, 0" "0.500000,0.500000,0.500000") "Undefined" "MultiplyWithRoot" 0 0))
    (Default|Move1 _returnvalue_2))
  (CallFunction|SpawnSurvive)
  (CallFunction|SpawnStaticCatches)
  (Components|DestroyComponent (Variables|Default|GetExitHard))
  (Components|DestroyComponent (Variables|Default|GetExitLight)))

(event OnComponentBeginOverlap(ExitLight)
  (params (OverlappedComponent :type Primitive%20Component%20Object%20Reference) (OtherActor :type Actor%20Object%20Reference) (OtherComp :type Primitive%20Component%20Object%20Reference) (OtherBodyIndex :type Integer) (bFromSweep :type Boolean) (SweepResult :type Hit%20Result%20Structure%20%28by%20ref%29))
  (bind _returnvalue (Transformation|GetActorLocation))
  (bind _x (Math|Vector|BreakVector _returnvalue))
  (Utilities|Casting|CastToBP_ThirdPersonCharacter OtherActor)
  (Variables|Default|SetCatchCount 6)
  (for _index (range 0 (- (Variables|Default|GetCatchCount) 1))
    (bind _returnvalue_2 (Game|SpawnActorfromClass "/Game/Blueprints/BP_First.BP_First_C" (Math|Transform|MakeTransform (Math|Vector|MakeVector (Math|Random|RandomFloatinRange (+ _x 1.15e+03) (+ _x 2.65e+03)) -3.2e+02 35.0) "0, 0, 0" "0.500000,0.500000,0.500000") "Undefined" "MultiplyWithRoot" 0 0))
    (Default|MoveSlow _returnvalue_2))
  (CallFunction|SpawnStaticCatches)
  (Components|DestroyComponent (Variables|Default|GetExitLight))
  (Components|DestroyComponent (Variables|Default|GetExitHard)))

(event OnComponentBeginOverlap(Stop1)
  (params (OverlappedComponent :type Primitive%20Component%20Object%20Reference) (OtherActor :type Actor%20Object%20Reference) (OtherComp :type Primitive%20Component%20Object%20Reference) (OtherBodyIndex :type Integer) (bFromSweep :type Boolean) (SweepResult :type Hit%20Result%20Structure%20%28by%20ref%29))
  (Utilities|Casting|CastToBP_ThirdPersonCharacter OtherActor)
  (Game|SpawnActorfromClass "/Game/Blueprints/BP_Block.BP_Block_C" (Math|Transform|MakeTransform (Math|Vector|MakeVector (+ (.X (Math|Vector|BreakVector (Transformation|GetActorLocation))) -5e+02) -3e+02 0.0) "0.000000,90.000000,0.000000" "1.000000,2.000000,1.000000") "Undefined" "MultiplyWithRoot" 0 0))

(event OnComponentBeginOverlap(Stop2)
  (params (OverlappedComponent :type Primitive%20Component%20Object%20Reference) (OtherActor :type Actor%20Object%20Reference) (OtherComp :type Primitive%20Component%20Object%20Reference) (OtherBodyIndex :type Integer) (bFromSweep :type Boolean) (SweepResult :type Hit%20Result%20Structure%20%28by%20ref%29))
  (Utilities|Casting|CastToBP_ThirdPersonCharacter OtherActor)
  (Game|SpawnActorfromClass "/Game/Blueprints/BP_Block.BP_Block_C" (Math|Transform|MakeTransform (Math|Vector|MakeVector (+ (.X (Math|Vector|BreakVector (Transformation|GetActorLocation))) -5e+02) -3e+02 0.0) "0.000000,90.000000,0.000000" "1.000000,2.000000,1.000000") "Undefined" "MultiplyWithRoot" 0 0))

(event EventBeginPlay)

(event Collision|EventActorBeginOverlap
  (params (OtherActor :type Actor%20Object%20Reference)))

(event EventTick
  (params (DeltaSeconds :type Float%20%28single-precision%29)))

(fn ConstructionScript)

(fn SpawnSurvive
  (bind _returnvalue (Transformation|GetActorLocation))
  (bind _x (Math|Vector|BreakVector _returnvalue))
  (Game|SpawnActorfromClass "/Game/Blueprints/BP_Survive.BP_Survive_C" (Math|Transform|MakeTransform (Math|Vector|MakeVector (Math|Random|RandomFloatinRange (+ _x 1.15e+03) (+ _x 2.65e+03)) (Math|Random|RandomFloatinRange -3.2e+02 4.5e+02) 1e+02)) "Undefined" "MultiplyWithRoot" 0 0))

(fn SpawnStaticCatches
  (bind _returnvalue (Transformation|GetActorLocation))
  (bind _x (Math|Vector|BreakVector _returnvalue))
  (for _index (range 0 (- (Variables|Default|GetCatchCount) 1))
    (Game|SpawnActorfromClass "/Game/Blueprints/BP_static_catch.BP_static_catch_C" (Math|Transform|MakeTransform (Math|Vector|MakeVector (Math|Random|RandomFloatinRange (+ _x 1.15e+03) (+ _x 2.65e+03)) (Math|Random|RandomFloatinRange -3.2e+02 4.5e+02) 35.0) "0, 0, 0" "0.500000,0.500000,0.500000") "Undefined" "MultiplyWithRoot" 0 0)))