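; BP_First is a moving hazard actor that calls TakeHarm with its Harm value on any BP_ThirdPersonCharacter entering its Box.
; Move1 and MoveSlow set endpoints from the current location plus a Target offset, then start ChangeLocation or NewMove, each lerping the actor on its own timeline.
; A FlipFlop re-triggered on timeline finish alternates play and reverse for continuous back-and-forth motion.
; MoveVerySlow only sets endpoints, and BeginPlay starts no movement.
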(event OnComponentBeginOverlap(Box)
  (params (OverlappedComponent :type Primitive%20Component%20Object%20Reference) (OtherActor :type Actor%20Object%20Reference) (OtherComp :type Primitive%20Component%20Object%20Reference) (OtherBodyIndex :type Integer) (bFromSweep :type Boolean) (SweepResult :type Hit%20Result%20Structure%20%28by%20ref%29))
  (bind _asbp_third_person_character (Utilities|Casting|CastToBP_ThirdPersonCharacter OtherActor))
  (Default|TakeHarm _asbp_third_person_character (Variables|Default|GetHarm)))

(event Custom|NewMove
  (Utilities|FlowControl|FlipFlop
    (:A
      (bind _betta (Timeline|Timeline_1 Play)
        (:Update
          (Transformation|SetActorLocation (Math|Vector|Lerp(Vector) (Variables|Default|GetPlace%20A) (Variables|Default|GetPlace%20B) _betta) false false))
        (:Finished
          (CallFunction|NewMove))))
    (:B
      (Timeline|Timeline_1 ReverseFromEnd))))

(event Custom|ChangeLocation
  (Utilities|FlowControl|FlipFlop
    (:A
      (bind _alpha (Timeline|Timeline Play)
        (:Update
          (Transformation|SetActorLocation (Math|Vector|Lerp(Vector) (Variables|Default|GetPlace%20A) (Variables|Default|GetPlace%20B) _alpha) false false))
        (:Finished
          (CallFunction|ChangeLocation))))
    (:B
      (Timeline|Timeline ReverseFromEnd))))

(event Custom|MoveSlow
  (Variables|Default|SetPlace%20A (Transformation|GetActorLocation))
  (Variables|Default|SetPlace%20B (+ (Variables|Default|GetPlace%20A) (Variables|Default|GetTarget)))
  (CallFunction|NewMove))

(event Custom|MoveVerySlow
  (Variables|Default|SetPlace%20A (Transformation|GetActorLocation))
  (Variables|Default|SetPlace%20B (+ (Variables|Default|GetPlace%20A) (Variables|Default|GetTarget))))

(event Custom|Move1
  (Variables|Default|SetPlace%20A (Transformation|GetActorLocation))
  (Variables|Default|SetPlace%20B (+ (Variables|Default|GetPlace%20A) (Variables|Default|GetTarget)))
  (CallFunction|ChangeLocation))

(event EventBeginPlay)

(event Collision|EventActorBeginOverlap
  (params (OtherActor :type Actor%20Object%20Reference)))

(event EventTick
  (params (DeltaSeconds :type Float%20%28single-precision%29)))

(fn ConstructionScript)